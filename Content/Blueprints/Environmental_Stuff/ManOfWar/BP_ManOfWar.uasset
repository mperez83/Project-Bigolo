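; BP_ManOfWar is an AI-controlled enemy that targets the player for chasing.
; On BeginPlay it caches its BP_ManOfWarController and an anim instance cast to the player's third-person AnimBP, then polls every 0.2 seconds until the player character exists.
; StartChasingPlayer writes that character to the TargetPlayer blackboard key, leaving the chase behavior outside this Blueprint.
; KillPlayer is an empty stub.
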(event `self.ReceiveBeginPlay`
  (bind _returnvalue (`GameplayStatics.GetPlayerCharacter` 0))
  (`|ExecutionSequence`
    (:`then_0`
      (set `self.AIController` (cast `/Game/Blueprints/Environmental_Stuff/ManOfWar/BP_ManOfWarController` (`self.GetController`) :!pure true))
      (set `self.AnimBP` (cast `/Game/Blueprints/Player/AnimBP_PlayerTPP` (`SkeletalMeshComponent.GetAnimInstance` (`self.Mesh`)) :!pure true)))
    (:`then_1`
      (`/Engine/EditorBlueprintResources/StandardMacros.IsValid` _returnvalue :!label _label
        (:`Is Valid`
          (`self.StartChasingPlayer` _returnvalue))
        (:`Is Not Valid`
          (`KismetSystemLibrary.Delay` 0.2)
          (goto _label))))))

(fn `KillPlayer`)

(fn `StartChasingPlayer`
  (params (PlayerToChase :type "Actor Object Reference"))
  (`BlackboardComponent.SetValueAsObject` (`AIBlueprintHelperLibrary.GetBlackboard` (`self.AIController`)) "TargetPlayer" PlayerToChase))

(fn `UserConstructionScript`)