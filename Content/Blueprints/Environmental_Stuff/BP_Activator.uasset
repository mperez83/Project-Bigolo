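; BP_Activator is an interactable object, built around a cube mesh, that toggles other actors in the environment.
; On interact it loops through its ActivatableActors array and calls OnToggle on each one.
; Look-at events switch the cube's Render Custom Depth on while the object is looked at and off when the look ends.
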(event `/Game/Blueprints/Player/BPI_Interactable.OnInteract`
  (params (CharacterReference :type "/Game/Blueprints/Player/MainPlayerCharacter Object Reference") (ControllerReference :type "/Game/Blueprints/Player/MainPlayerController Object Reference") (AtypicalInteract :type Boolean))
  (for _array_element (`self.ActivatableActors`)
    (`/Game/Blueprints/Player/BPI_Activatable.OnToggle` _array_element)))

(event `/Game/Blueprints/Player/BPI_Interactable.OnLookAtStart`
  (`PrimitiveComponent.SetRenderCustomDepth` (`self.Cube`) true))

(event `/Game/Blueprints/Player/BPI_Interactable.OnLookAtTick`
  (bind _cube (`self.Cube`))
  (if (not (`PrimitiveComponent.bRenderCustomDepth` _cube))
    (`PrimitiveComponent.SetRenderCustomDepth` _cube true)))

(event `/Game/Blueprints/Player/BPI_Interactable.OnLookAtEnd`
  (`PrimitiveComponent.SetRenderCustomDepth` (`self.Cube`) false))

(fn `UserConstructionScript`)