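; World text actor that reveals a widget label when the local player's camera comes within a set distance.
; Tick compares camera distance and, optionally, line of sight from a trace against WorldStatic objects.
; Crossing either condition toggles the shown flag on the W_WorldText widget and plays its Reveal animation forward or in reverse.
; A RepNotify on Text pushes replicated text changes into the widget.
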(event `self.ReceiveBeginPlay`
  (set `self.WorldTextRef` (cast `/Game/UI/W_WorldText` (`WidgetComponent.GetWidget` (`self.WorldTextWidget`)) :!pure true)))

(event `self.ReceiveTick`
  (params (DeltaSeconds :type "Float (single-precision)"))
  (bind _worldtextref (`self.WorldTextRef`))
  (bind _worldtextref_2 (`self.WorldTextRef`))
  (bind _returnvalue (< (`KismetMathLibrary.Vector_Distance` (`PlayerCameraManager.GetCameraLocation` (`GameplayStatics.GetPlayerCameraManager` 0)) (`self.K2_GetActorLocation`)) (`self.DistanceTextIsShown`)))
  (if (`/Game/UI/W_WorldText.TextIsShown` _worldtextref_2)
    (if _returnvalue
      (if (`self.LineOfSightRequired`)
        (if (not (`self.GetIfHasLineOfSightWithPlayer`))
          (set `/Game/UI/W_WorldText.TextIsShown` false _worldtextref_2 :!label _label)
          (`UserWidget.PlayAnimation` _worldtextref_2 (`/Game/UI/W_WorldText.Reveal` _worldtextref_2) 0.0 1 "Reverse" 1.0 false)))
      (else
        (goto _label)))
    (elif _returnvalue
      (if (`self.LineOfSightRequired`)
        (if (`self.GetIfHasLineOfSightWithPlayer`)
          (set `/Game/UI/W_WorldText.TextIsShown` true _worldtextref :!label _label_2)
          (`UserWidget.PlayAnimation` _worldtextref (`/Game/UI/W_WorldText.Reveal` _worldtextref) 0.0 1 "Forward" 1.0 false))
        (else
          (goto _label_2))))))

(fn `GetIfHasLineOfSightWithPlayer`
  (returns (HasLineOfSight :type Boolean))
  (bind (_outhit _returnvalue) (`KismetSystemLibrary.LineTraceSingleForObjects` (`PlayerCameraManager.GetCameraLocation` (`GameplayStatics.GetPlayerCameraManager` 0)) (`self.K2_GetActorLocation`) (`|MakeArray` "ObjectTypeQuery1" :!type "EObjectTypeQuery Enum")))
  (return (not _returnvalue)))

(fn `OnRep_Text`
  (`self.SetWTText` (`self.Text`)))

(fn `SetWTText`
  (params (NewText :type Text))
  (bind _worldtextref (`self.WorldTextRef`)
    (:`then`
      (`TextBlock.SetText` (`/Game/UI/W_WorldText.Text` _worldtextref) NewText))
    (:`else`)))

(fn `UserConstructionScript`)