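; Base interactable actor with a skeletal mesh that players can look at and interact with, optionally using their selected item.
; Custom depth outlines follow an outline mode, driven by look-at events and interactable state, which also toggles the interact box's collision.
; A successful TryInteract can drop the selected item at the mesh (optionally unpickuppable) or destroy it.
; It can also reveal the mesh in the main pass, then calls OnInteracted.
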(event `self.ReceiveBeginPlay`
  (`self.SetIsInteractable` (`self.IsInteractable`))
  (switch `/Game/Blueprints/System/E_InteractableOutlineTypes` (`self.OutlineType`)
    (:`NewEnumerator1`
      (`PrimitiveComponent.SetRenderCustomDepth` (`self.SkeletalMesh`) true))))

(event `/Game/Blueprints/Player/BPI_Interactable.OnLookAtStart`
  (switch `/Game/Blueprints/System/E_InteractableOutlineTypes` (`self.OutlineType`)
    (:`NewEnumerator0`
      (if (`self.IsInteractable`)
        (`PrimitiveComponent.SetRenderCustomDepth` (`self.SkeletalMesh`) true)))))

(event `/Game/Blueprints/Player/BPI_Interactable.OnLookAtTick`
  (bind _skeletalmesh (`self.SkeletalMesh`))
  (switch `/Game/Blueprints/System/E_InteractableOutlineTypes` (`self.OutlineType`)
    (:`NewEnumerator0`
      (if (`self.IsInteractable`)
        (if (not (`PrimitiveComponent.bRenderCustomDepth` _skeletalmesh))
          (`PrimitiveComponent.SetRenderCustomDepth` _skeletalmesh true))))))

(event `/Game/Blueprints/Player/BPI_Interactable.OnLookAtEnd`
  (switch `/Game/Blueprints/System/E_InteractableOutlineTypes` (`self.OutlineType`)
    (:`NewEnumerator0`
      (`PrimitiveComponent.SetRenderCustomDepth` (`self.SkeletalMesh`) false))))

(event `/Game/Blueprints/Player/BPI_Interactable.OnInteract`
  (params (CharacterReference :type "/Game/Blueprints/Player/MainPlayerCharacter Object Reference") (ControllerReference :type "/Game/Blueprints/Player/MainPlayerController Object Reference") (AtypicalInteract :type Boolean))
  (bind _selecteditem (`/Game/Blueprints/Player/MainPlayerController.GetSelectedItem` ControllerReference))
  (bind _success (`self.TryInteract` CharacterReference ControllerReference AtypicalInteract))
  (if _success
    (`|ExecutionSequence`
      (:`then_0`
        (switch `/Game/Blueprints/System/E_InteractableItemUseBehaviour` (`self.ItemUseBehaviour`)
          (:`NewEnumerator1`
            (`/Game/Blueprints/Player/MainPlayerController.ServerDropItem` ControllerReference _selecteditem (`KismetMathLibrary.MakeTransform` (`SceneComponent.K2_GetComponentLocation` (`self.SkeletalMesh`))) (0.0 0.0 0.0) :!label _label))
          (:`NewEnumerator3`
            (set `/Game/Blueprints/Items/Item_Base.Pickuppable` false _selecteditem)
            (goto _label))
          (:`NewEnumerator2`
            (`/Game/Blueprints/Player/MainPlayerController.RemoveItem` ControllerReference _selecteditem true))))
      (:`then_1`
        (if (`self.MakeMeshVisibleOnInteract`)
          (`self.SetRenderMainPass` true)))
      (:`then_2`
        (`self.OnInteracted` CharacterReference ControllerReference)))))

(fn `SetIsInteractable`
  (params (IsInteractable :type Boolean))
  (bind _output_get (set `self.IsInteractable` IsInteractable))
  (if _output_get
    (`PrimitiveComponent.SetCollisionEnabled` (`self.InteractBox`) "QueryOnly")
    (switch `/Game/Blueprints/System/E_InteractableOutlineTypes` (`self.OutlineType`)
      (:`NewEnumerator3`
        (`PrimitiveComponent.SetRenderCustomDepth` (`self.SkeletalMesh`) true)))
    (else
      (`PrimitiveComponent.SetCollisionEnabled` (`self.InteractBox`) "NoCollision")
      (switch `/Game/Blueprints/System/E_InteractableOutlineTypes` (`self.OutlineType`)
        (:`NewEnumerator0`
          _)
        (:`NewEnumerator3`
          _))
      (`PrimitiveComponent.SetRenderCustomDepth` (`self.SkeletalMesh`) false))))

(fn `SetRenderMainPass`
  (params (RenderMainPass :type Boolean))
  (`PrimitiveComponent.SetRenderInMainPass` (`self.SkeletalMesh`) RenderMainPass))

(fn `UserConstructionScript`
  (`parent.UserConstructionScript`))