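; Interactable static-mesh actor that players can look at and use, optionally requiring a specific selected inventory item.
; A configurable outline type toggles the mesh's custom depth from look-at events and interactable state changes.
; On a valid interaction, a required item is dropped at the mesh (optionally made unpickuppable) or destroyed, and the mesh can be revealed.
; Successful interactions, with or without a required item, fire OnInteracted with the character and controller.
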(event `self.ReceiveBeginPlay`
  (`self.SetIsInteractable` (`self.IsInteractable`))
  (switch `/Game/Blueprints/System/E_InteractableOutlineTypes` (`self.OutlineType`)
    (:`NewEnumerator1`
      (`PrimitiveComponent.SetRenderCustomDepth` (`self.StaticMesh`) true))))

(event `/Game/Blueprints/Player/BPI_Interactable.OnLookAtStart`
  (switch `/Game/Blueprints/System/E_InteractableOutlineTypes` (`self.OutlineType`)
    (:`NewEnumerator0`
      (if (`self.IsInteractable`)
        (`PrimitiveComponent.SetRenderCustomDepth` (`self.StaticMesh`) true)))))

(event `/Game/Blueprints/Player/BPI_Interactable.OnLookAtTick`
  (bind _staticmesh (`self.StaticMesh`))
  (switch `/Game/Blueprints/System/E_InteractableOutlineTypes` (`self.OutlineType`)
    (:`NewEnumerator0`
      (if (`self.IsInteractable`)
        (if (not (`PrimitiveComponent.bRenderCustomDepth` _staticmesh))
          (`PrimitiveComponent.SetRenderCustomDepth` _staticmesh true))))))

(event `/Game/Blueprints/Player/BPI_Interactable.OnLookAtEnd`
  (switch `/Game/Blueprints/System/E_InteractableOutlineTypes` (`self.OutlineType`)
    (:`NewEnumerator0`
      (`PrimitiveComponent.SetRenderCustomDepth` (`self.StaticMesh`) false))))

(event `/Game/Blueprints/Player/BPI_Interactable.OnInteract`
  (params (CharacterReference :type "/Game/Blueprints/Player/MainPlayerCharacter Object Reference") (ControllerReference :type "/Game/Blueprints/Player/MainPlayerController Object Reference") (AtypicalInteract :type Boolean))
  (bind _selecteditem (`/Game/Blueprints/Player/MainPlayerController.GetSelectedItem` ControllerReference))
  (if (`self.IsInteractable`)
    (if (`KismetSystemLibrary.IsValid` (`self.RequiredItem`))
      (if (== (`self.RequiredItem`) _selecteditem)
        (`|ExecutionSequence`
          (:`then_0`
            (switch `/Game/Blueprints/System/E_InteractableItemUseBehaviour` (`self.ItemUseBehaviour`)
              (:`NewEnumerator1`
                (`/Game/Blueprints/Player/MainPlayerController.ServerDropItem` ControllerReference _selecteditem (`KismetMathLibrary.MakeTransform` (`SceneComponent.K2_GetComponentLocation` (`self.StaticMesh`)) (struct)) (0.0 0.0 0.0) :!label _label))
              (:`NewEnumerator3`
                (set `/Game/Blueprints/Items/Item_Base.Pickuppable` false _selecteditem)
                (goto _label))
              (:`NewEnumerator2`
                (`/Game/Blueprints/Player/MainPlayerController.RemoveItem` ControllerReference _selecteditem true))))
          (:`then_1`
            (if (`self.MakeMeshVisibleOnInteract`)
              (`PrimitiveComponent.SetRenderInMainPass` (`self.StaticMesh`) true)))
          (:`then_2`
            (`self.OnInteracted` CharacterReference ControllerReference :!label _label_2))))
      (else
        (goto _label_2)))))

(fn `SetIsInteractable`
  (params (IsInteractable :type Boolean))
  (bind _output_get (set `self.IsInteractable` IsInteractable))
  (if _output_get
    (switch `/Game/Blueprints/System/E_InteractableOutlineTypes` (`self.OutlineType`)
      (:`NewEnumerator3`
        (`PrimitiveComponent.SetRenderCustomDepth` (`self.StaticMesh`) true)))
    (else
      (switch `/Game/Blueprints/System/E_InteractableOutlineTypes` (`self.OutlineType`)
        (:`NewEnumerator0`
          _)
        (:`NewEnumerator3`
          _))
      (`PrimitiveComponent.SetRenderCustomDepth` (`self.StaticMesh`) false))))

(fn `UserConstructionScript`
  (`parent.UserConstructionScript`))