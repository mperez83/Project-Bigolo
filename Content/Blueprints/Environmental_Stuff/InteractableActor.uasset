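; Interactable actor that provides a common gate for player interaction, apparently as a base for environmental objects.
; TryInteract succeeds only when the actor is interactable and, if a valid RequiredItem is set, the controller's selected item matches it.
; It only returns that result; CharacterRef and ATypicalInteract go unused here.
; SetIsInteractable and SetRenderMainPass are empty stubs, as is the construction script.
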(fn `SetIsInteractable`
  (params (IsInteractable :type Boolean)))

(fn `SetRenderMainPass`
  (params (RenderMainPass :type Boolean)))

(fn `TryInteract`
  (params (CharacterRef :type "/Game/Blueprints/Player/MainPlayerCharacter Object Reference") (ControllerRef :type "/Game/Blueprints/Player/MainPlayerController Object Reference") (ATypicalInteract :type Boolean))
  (returns (Success :type Boolean))
  (if (`self.IsInteractable`)
    (if (`KismetSystemLibrary.IsValid` (`self.RequiredItem`))
      (if (== (`self.RequiredItem`) (`/Game/Blueprints/Player/MainPlayerController.GetSelectedItem` ControllerRef))
        (return true)
        (else
          _))
      (else
        (return true))))
  (return false))

(fn `UserConstructionScript`)