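; Interactable hinged door that plays sounds and can be locked, in which case interacting only jiggles the knob.
; Opening chains a knob-turn timeline into a swing timeline that lerps pivot yaw to OpenAngle, with play rates derived from duration variables.
; Interacting while open reverses the swing, even mid-motion, and input is blocked during the knob turn.
; A temporary door previews the open angle via the construction script and is destroyed at BeginPlay.
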(event `self.ReceiveBeginPlay`
  (`ActorComponent.K2_DestroyComponent` (`self.TempDoor`))
  (`ActorComponent.K2_DestroyComponent` (`self.TempDoorPivot`))
  (`TimelineComponent.SetPlayRate` (`self.DoorOpenAnimTL`) (/ 1.0 (`self.DoorSwingTime`)))
  (`TimelineComponent.SetPlayRate` (`self.DoorKnobOpenAnimTL`) (/ 1.0 (`self.DoorKnobTurnTime`))))

(event `/Game/Blueprints/Player/BPI_Interactable.OnInteract`
  (params (CharacterReference :type "/Game/Blueprints/Player/MainPlayerCharacter Object Reference") (ControllerReference :type "/Game/Blueprints/Player/MainPlayerController Object Reference") (AtypicalInteract :type Boolean))
  (bind _doorknobjiggleanimtl (`self.DoorKnobJiggleAnimTL`))
  (if (`self.CanInteract`)
    (if (`self.Locked`)
      (`GameplayStatics.PlaySoundAtLocation` "/Game/Audio/Environment_Audio/S_DoorLocked_Cue.S_DoorLocked_Cue" (`SceneComponent.K2_GetComponentLocation` (`self.DoorKnob`)) (struct) 1.0 1.0 0.0 null null null)
      (if (not (`TimelineComponent.IsPlaying` _doorknobjiggleanimtl))
        (`TimelineComponent.PlayFromStart` _doorknobjiggleanimtl))
      (elif (`self.Open`)
        (switch `ETimelineDirection` (`self.DoorOpenAnimTLDirection`)
          (:`Forward`
            (`TimelineComponent.Reverse` (`self.DoorOpenAnimTL`)))
          (:`Backward`
            (`TimelineComponent.Play` (`self.DoorOpenAnimTL`))))
        (else
          (`TimelineComponent.PlayFromStart` (`self.DoorKnobOpenAnimTL`))
          (`GameplayStatics.PlaySoundAtLocation` "/Game/Audio/Environment_Audio/S_DoorOpen_Cue.S_DoorOpen_Cue" (`SceneComponent.K2_GetComponentLocation` (`self.DoorKnob`)) (struct) 1.0 1.0 0.0 null null null)
          (set `self.CanInteract` false))))))

(fn `UserConstructionScript`
  (`SceneComponent.K2_SetRelativeRotation` (`self.TempDoorPivot`) (`KismetMathLibrary.MakeRotator` 0.0 0.0 (`self.OpenAngle`)) false false))