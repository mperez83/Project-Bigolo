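; BP_TV is an interactable television prop that toggles on and off.
; Interacting flips its Activated state, swapping the Screen material between TV static and unlit black while starting or stopping the StaticAudio sound.
; Look-at events toggle custom depth rendering on the Base mesh while the TV is looked at, with the tick event re-enabling it if it is off.
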(event `/Game/Blueprints/Player/BPI_Interactable.OnInteract`
  (params (CharacterReference :type "/Game/Blueprints/Player/MainPlayerCharacter Object Reference") (ControllerReference :type "/Game/Blueprints/Player/MainPlayerController Object Reference") (AtypicalInteract :type Boolean))
  (`self.OnToggle`))

(event `self.OnToggle`
  (if (`self.Activated`)
    (`self.OnDeactivate`)
    (else
      (`self.OnActivate`))))

(event `self.OnActivate`
  (set `self.Activated` true)
  (`PrimitiveComponent.SetMaterial` (`self.Screen`) 0 "/Game/Graphics/Materials/M_TVStatic.M_TVStatic")
  (`AudioComponent.Play` (`self.StaticAudio`) 0.0))

(event `self.OnDeactivate`
  (set `self.Activated` false)
  (`PrimitiveComponent.SetMaterial` (`self.Screen`) 0 "/Engine/EngineDebugMaterials/BlackUnlitMaterial.BlackUnlitMaterial")
  (`AudioComponent.Stop` (`self.StaticAudio`)))

(event `/Game/Blueprints/Player/BPI_Interactable.OnLookAtStart`
  (`PrimitiveComponent.SetRenderCustomDepth` (`self.Base`) true))

(event `/Game/Blueprints/Player/BPI_Interactable.OnLookAtTick`
  (bind _base (`self.Base`))
  (if (not (`PrimitiveComponent.bRenderCustomDepth` _base))
    (`PrimitiveComponent.SetRenderCustomDepth` _base true)))

(event `/Game/Blueprints/Player/BPI_Interactable.OnLookAtEnd`
  (`PrimitiveComponent.SetRenderCustomDepth` (`self.Base`) false))

(fn `UserConstructionScript`)