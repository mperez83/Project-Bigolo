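; Main game state Blueprint that resets interactables and daily chores on day changes and offers shared sound and particle events.
; SetDayNum runs the same reset for days two through four: it disables every InteractableActor, hides from the main render pass those that reveal their mesh on interaction, and resets the TaskDailyChores actor.
; Separate Multi-prefixed events, apparently multicasts, play a sound or spawn an emitter at a location.
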(event `MultiPlaySoundAtLocation`
  (params (Sound :type "SoundBase Object Reference") (Location :type "Vector Structure"))
  (`GameplayStatics.PlaySoundAtLocation` Sound Location (struct) 1.0 1.0 0.0 null null null))

(event `MultiSpawnEmitterAtLocation`
  (params (EmitterTemplate :type "ParticleSystem Object Reference") (SpawnTransform :type "Transform Structure"))
  (`GameplayStatics.SpawnEmitterAtLocation` EmitterTemplate SpawnTransform_Location SpawnTransform_Rotation SpawnTransform_Scale))

(fn `SetDayNum`
  (params (NewDayNum :type Integer))
  (switch `int` NewDayNum
    (:`2`
      _)
    (:`3`
      _)
    (:`4`
      _))
  (`|ExecutionSequence`
    (:`then_0`
      (bind _outactors (`GameplayStatics.GetAllActorsOfClass` "/Game/Blueprints/Environmental_Stuff/InteractableActor.InteractableActor_C"))
      (for _array_element _outactors
        (`/Game/Blueprints/Environmental_Stuff/InteractableActor.SetIsInteractable` _array_element false)
        (if (`/Game/Blueprints/Environmental_Stuff/InteractableActor.MakeMeshVisibleOnInteract` _array_element)
          (`/Game/Blueprints/Environmental_Stuff/InteractableActor.SetRenderMainPass` _array_element false))))
    (:`then_1`
      (bind _returnvalue (`GameplayStatics.GetActorOfClass` "/Game/Blueprints/System/TaskStuff/Tasks/TaskDailyChores.TaskDailyChores_C"))
      (`/Game/Blueprints/System/TaskStuff/Tasks/TaskBase.ResetTask` _returnvalue))))

(fn `UserConstructionScript`)