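; Base class for replicated pickup items that players add to the hotbar, equip and drop, with empty action hooks.
; RepNotifies on PlayerRef, Active, Frozen, Pickuppable and NewMesh drive attachment, visibility, physics, collision and mesh swaps.
; Separate world, first-person and third-person meshes serve dropped and held states, with equipping setting the owner's FPP animations.
; It also handles custom-depth outlines, material override and restore, and throttled impact sounds by surface type.
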(event `self.ReceiveBeginPlay`
  (set `self.GameStateRef` (cast `/Game/Blueprints/System/MainGameState` (`GameplayStatics.GetGameState`) :!pure true))
  (`/Engine/EditorBlueprintResources/ActorMacros.Switch Has Authority`
    (:`Authority`
      (set `self.PlayerRef` (`self.PlayerRef`))
      (set `self.Frozen` (`self.Frozen`)))))

(event `DropItem`
  (params (SpawnTransform :type "Transform Structure") (DropForce :type "Vector Structure"))
  (bind _worldmesh (`self.WorldMesh`))
  (`SceneComponent.K2_SetWorldTransform` _worldmesh (`KismetMathLibrary.MakeTransform` SpawnTransform_Location SpawnTransform_Rotation (`SceneComponent.K2_GetComponentScale` _worldmesh)) false true)
  (`self.OnUnequip`)
  (`self.OnDrop`)
  (set `self.MPC` null)
  (set `self.PlayerRef` null)
  (set `self.Active` false)
  (`SkeletalMeshComponent.AddImpulseToAllBodiesBelow` _worldmesh DropForce "None" true true))

(event `/Game/Blueprints/Player/BPI_Interact.OnInteract`
  (params (CharacterReference :type "/Game/Blueprints/Player/MainPlayerCharacter Object Reference") (ControllerReference :type "/Game/Blueprints/Player/MainPlayerController Object Reference") (AtypicalInteract :type Boolean))
  (`|ExecutionSequence`
    (:`then_0`
      (`self.OnInteracted`))
    (:`then_1`
      (if (`self.Pickuppable`)
        (set `self.Frozen` false)
        (bind _emptyslotindex (`/Game/Blueprints/Player/MainPlayerController.FindEmptyHotbarSlot` ControllerReference))
        (if (!= _emptyslotindex -1)
          (`self.ForceNetUpdate`)
          (`/Game/Blueprints/Player/MainPlayerController.AddAndEquipItem` ControllerReference self))))))

(event `/Game/Blueprints/Player/BPI_Interact.EnableOutline`
  (params (Enabled :type Boolean))
  (bind _worldmesh (`self.WorldMesh`))
  (if Enabled
    (if (not (`PrimitiveComponent.bRenderCustomDepth` _worldmesh))
      (`PrimitiveComponent.SetRenderCustomDepth` _worldmesh true))
    (elif (`PrimitiveComponent.bRenderCustomDepth` _worldmesh)
      (`PrimitiveComponent.SetRenderCustomDepth` _worldmesh false))))

(event `OwningClientSetFPPAnimations`
  (bind _playerref (`self.PlayerRef`)
    (:`then`
      (bind _fppanimbp (`/Game/Blueprints/Player/MainPlayerCharacter.FPPAnimBP` _playerref)
        (:`then`
          (`/Game/Blueprints/Player/AnimBP_PlayerFPP.SetAllAnimations` _fppanimbp (`self.IdleAnim`) (`self.WalkAnim`) (`self.SprintAnim`) (`self.JumpStartAnim`) (`self.JumpLoopAnim`) (`self.JumpEndAnim`))
          (`AnimInstance.Montage_Play` _fppanimbp (`self.EquipAnim`) 1.0 "MontageLength" 0.0 true))
        (:`else`)))
    (:`else`)))

(event `MultiPlaySoundAtLocation`
  (params (Sound :type "SoundBase Object Reference") (Location :type "Vector Structure"))
  (`GameplayStatics.PlaySoundAtLocation` Sound Location (struct) 1.0 1.0 0.0 null null null))

(event `OnActorHitPhysicsNoiseCheck`
  (params (SelfActor :type "Actor Object Reference") (OtherActor :type "Actor Object Reference") (NormalImpulse :type "Vector Structure") (Hit :type "HitResult Structure (by ref)"))
  (if (> (`KismetMathLibrary.VSize` NormalImpulse) 30000.0)
    (`/Engine/EditorBlueprintResources/StandardMacros.DoOnce` false :!label _label
      (:`Completed`
        (`|ExecutionSequence`
          (:`then_0`
            (switch `/Game/Blueprints/Items/E_ItemCollisionSoundType` (`self.CollisionSoundType`)
              (:`NewEnumerator0`
                (`GameplayStatics.PlaySoundAtLocation` "/Game/Audio/Item_Audio/Impact_Audio/Impact_Generic_Cue.Impact_Generic_Cue" Hit_Location (struct) 1.0 1.0 0.0 null null null))
              (:`NewEnumerator1`
                (`GameplayStatics.PlaySoundAtLocation` "/Game/Audio/Item_Audio/Impact_Audio/Impact_Wood_Cue.Impact_Wood_Cue" Hit_Location (struct) 1.0 1.0 0.0 null null null))
              (:`NewEnumerator2`
                (`GameplayStatics.PlaySoundAtLocation` "/Game/Audio/Item_Audio/Impact_Audio/Impact_Gun_Cue.Impact_Gun_Cue" Hit_Location (struct) 1.0 1.0 0.0 null null null))
              (:`NewEnumerator3`
                (`GameplayStatics.PlaySoundAtLocation` "/Game/Audio/Item_Audio/Impact_Audio/Impact_Flesh_Cue.Impact_Flesh_Cue" Hit_Location (struct) 1.0 1.0 0.0 null null null))
              (:`NewEnumerator4`
                (`GameplayStatics.PlaySoundAtLocation` "/Game/Audio/Item_Audio/Impact_Audio/Impact_Metal_Cue.Impact_Metal_Cue" (0.0 0.0 0.0) (struct) 1.0 1.0 0.0 null null null))))
          (:`then_1`
            (`KismetSystemLibrary.Delay` 0.2)
            (goto _label :!via `Reset`)))))))

(fn `DisableItemStuff`
  (bind _worldmesh (`self.WorldMesh`))
  (`self.SetActorHiddenInGame` false)
  (`SceneComponent.SetHiddenInGame` (`self.FPP_ItemMesh`) true true)
  (`SceneComponent.SetHiddenInGame` (`self.TPP_ItemMesh`) true true)
  (`SceneComponent.SetHiddenInGame` _worldmesh false false)
  (`PrimitiveComponent.SetSimulatePhysics` _worldmesh true)
  (`PrimitiveComponent.SetCollisionEnabled` _worldmesh "QueryAndPhysics")
  (`PrimitiveComponent.SetCollisionEnabled` (`self.Box`) "QueryOnly")
  (`self.K2_DetachFromActor` "KeepRelative"))

(fn `EnableItemStuff`
  (bind _playerref (`self.PlayerRef`))
  (bind _fpp_itemmesh (`self.FPP_ItemMesh`))
  (bind _tpp_itemmesh (`self.TPP_ItemMesh`))
  (bind _worldmesh (`self.WorldMesh`))
  (`SceneComponent.SetHiddenInGame` (`self.FPP_ItemMesh`) false true)
  (`SceneComponent.SetHiddenInGame` (`self.TPP_ItemMesh`) false true)
  (`SceneComponent.SetHiddenInGame` _worldmesh true false)
  (`PrimitiveComponent.SetSimulatePhysics` _worldmesh false)
  (`PrimitiveComponent.SetCollisionEnabled` _worldmesh "NoCollision")
  (`PrimitiveComponent.SetCollisionEnabled` (`self.Box`) "NoCollision")
  (`/Game/Blueprints/Player/MainPlayerCharacter.AttachItemToPlayer` _playerref self)
  (if (`Pawn.IsLocallyControlled` _playerref)
    (`|ExecutionSequence`
      (:`then_0`
        (`PrimitiveComponent.SetOnlyOwnerSee` _fpp_itemmesh true)
        (`PrimitiveComponent.SetOwnerNoSee` _fpp_itemmesh false))
      (:`then_1`
        (`PrimitiveComponent.SetOnlyOwnerSee` _tpp_itemmesh false)
        (`PrimitiveComponent.SetOwnerNoSee` _tpp_itemmesh true)))))

(fn `OnPrimaryAction`
  (params (Pressed :type Boolean))
  (return))

(fn `OnReloadAction`
  (params (Pressed :type Boolean))
  (return))

(fn `OnRep_Active`
  (`/Engine/EditorBlueprintResources/StandardMacros.IsValid` (`self.PlayerRef`)
    (:`Is Valid`
      (if (`self.Active`)
        (`self.SetActorHiddenInGame` false)
        (`self.OwningClientSetFPPAnimations`)
        (`self.OnEquip`)
        (else
          (`self.SetActorHiddenInGame` true)
          (`self.OnUnequip`))))))

(fn `OnRep_Frozen`
  (if (`self.Frozen`)
    (`PrimitiveComponent.SetSimulatePhysics` (`self.WorldMesh`) false)
    (`PrimitiveComponent.SetCollisionResponseToChannel` (`self.WorldMesh`) "ECC_Pawn" "ECR_Overlap")
    (else
      (`PrimitiveComponent.SetSimulatePhysics` (`self.WorldMesh`) true)
      (`PrimitiveComponent.SetCollisionResponseToChannel` (`self.WorldMesh`) "ECC_Pawn" "ECR_Block"))))

(fn `OnRep_NewMesh`
  (bind _newmesh (`self.NewMesh`))
  (`|ExecutionSequence`
    (:`then_0`
      (`SkinnedMeshComponent.SetSkinnedAssetAndUpdate` (`self.WorldMesh`) _newmesh true)
      (`SkinnedMeshComponent.SetSkinnedAssetAndUpdate` (`self.FPP_ItemMesh`) _newmesh true)
      (`SkinnedMeshComponent.SetSkinnedAssetAndUpdate` (`self.TPP_ItemMesh`) _newmesh true))
    (:`then_1`
      (for _array_element (`MeshComponent.GetMaterials` (`self.WorldMesh`))
        (`KismetArrayLibrary.Array_Add` (`self.OriginalMats`) _array_element)))
    (:`then_2`
      (`/Engine/EditorBlueprintResources/ActorMacros.Switch Has Authority`))))

(fn `OnRep_Pickuppable`
  (if (`self.Pickuppable`)
    (`PrimitiveComponent.SetCollisionEnabled` (`self.Box`) "QueryOnly")
    (else
      (`PrimitiveComponent.SetCollisionEnabled` (`self.Box`) "NoCollision"))))

(fn `OnRep_PlayerRef`
  (`self.V_OnRep_PlayerRef`))

(fn `OnSecondaryAction`
  (params (Pressed :type Boolean))
  (return))

(fn `SetAllMeshMats`
  (params (NewMat :type "MaterialInterface Object Reference"))
  (bind _tpp_itemmesh (`self.TPP_ItemMesh`))
  (bind _worldmesh (`self.WorldMesh`))
  (bind _fpp_itemmesh (`self.FPP_ItemMesh`))
  (`|ExecutionSequence`
    (:`then_0`
      (for (_ _array_index) (`MeshComponent.GetMaterials` _worldmesh)
        (`PrimitiveComponent.SetMaterial` _worldmesh _array_index NewMat)))
    (:`then_1`
      (for (_ _array_index_2) (`MeshComponent.GetMaterials` _fpp_itemmesh)
        (`PrimitiveComponent.SetMaterial` _fpp_itemmesh _array_index_2 NewMat)))
    (:`then_2`
      (for (_ _array_index_3) (`MeshComponent.GetMaterials` _tpp_itemmesh)
        (`PrimitiveComponent.SetMaterial` _tpp_itemmesh _array_index_3 NewMat)))))

(fn `SetOriginalMats`
  (bind _tpp_itemmesh (`self.TPP_ItemMesh`))
  (bind _worldmesh (`self.WorldMesh`))
  (bind _fpp_itemmesh (`self.FPP_ItemMesh`))
  (`|ExecutionSequence`
    (:`then_0`
      (for (_ _array_index) (`MeshComponent.GetMaterials` _worldmesh)
        (`PrimitiveComponent.SetMaterial` _worldmesh _array_index (`|GetArrayItem` (`self.OriginalMats`) _array_index))))
    (:`then_1`
      (for (_ _array_index_2) (`MeshComponent.GetMaterials` _fpp_itemmesh)
        (`PrimitiveComponent.SetMaterial` _fpp_itemmesh _array_index_2 (`|GetArrayItem` (`self.OriginalMats`) _array_index_2))))
    (:`then_2`
      (for (_ _array_index_3) (`MeshComponent.GetMaterials` _tpp_itemmesh)
        (`PrimitiveComponent.SetMaterial` _tpp_itemmesh _array_index_3 (`|GetArrayItem` (`self.OriginalMats`) _array_index_3))))))

(fn `SetOutline`
  (params (Enabled :type Boolean))
  (bind _tpp_itemmesh (`self.TPP_ItemMesh`))
  (if Enabled
    (if (not (`PrimitiveComponent.bRenderCustomDepth` _tpp_itemmesh))
      (`PrimitiveComponent.SetRenderCustomDepth` _tpp_itemmesh true))
    (elif (`PrimitiveComponent.bRenderCustomDepth` _tpp_itemmesh)
      (`PrimitiveComponent.SetRenderCustomDepth` _tpp_itemmesh false))))

(fn `UserConstructionScript`
  (for _array_element (`MeshComponent.GetMaterials` (`self.WorldMesh`))
    (`KismetArrayLibrary.Array_Add` (`self.OriginalMats`) _array_element)))

(fn `V_OnRep_PlayerRef`
  (`self.SetOwner` (`self.PlayerRef`))
  (`self.PlayerRef`
    (:`then`
      (`self.EnableItemStuff`))
    (:`else`
      (`self.DisableItemStuff`))))