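; Blueprint utility library of general helper functions for toggling actors and making random picks.
; DisableActor and EnableActor switch an actor's visibility in game, collision and tick together.
; PullStringFromTable and PullIntFromTable do weighted random selection, summing map values as weights, then subtracting along the keys until the roll lands.
; RandomChanceBool rolls against a percentage chance from 0 to 100.
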(fn `DisableActor`
  (params (ActorToDisable :type "Actor Object Reference"))
  (`Actor.SetActorHiddenInGame` ActorToDisable true)
  (`Actor.SetActorEnableCollision` ActorToDisable false)
  (`Actor.SetActorTickEnabled` ActorToDisable false))

(fn `EnableActor`
  (params (ActorToEnable :type "Actor Object Reference"))
  (`Actor.SetActorHiddenInGame` ActorToEnable false)
  (`Actor.SetActorEnableCollision` ActorToEnable true)
  (`Actor.SetActorTickEnabled` ActorToEnable true))

(fn `PullIntFromTable`
  (params (IntMap :type "Map of Integer to Float (double-precision)"))
  (returns (Return :type Integer))
  (locals (RunningSum :type "Float (double-precision)") (RandomVal :type "Float (double-precision)"))
  (bind _values (`BlueprintMapLibrary.Map_Values` IntMap))
  (for _array_element _values
    (set `local.RunningSum` (+ _array_element (`local.RunningSum`))))
  (set `local.RandomVal` (`KismetMathLibrary.RandomFloatInRange` 0.0 (`local.RunningSum`)))
  (bind _keys (`BlueprintMapLibrary.Map_Keys` IntMap))
  (for _array_element_2 _keys
    (bind _value (`BlueprintMapLibrary.Map_Find` IntMap _array_element_2))
    (if (< (`local.RandomVal`) _value)
      (return _array_element_2)
      (else
        (set `local.RandomVal` (- (`local.RandomVal`) _value))))))

(fn `PullStringFromTable`
  (params (StringMap :type "Map of String to Float (double-precision)"))
  (returns (Return :type String))
  (locals (RunningSum :type "Float (double-precision)") (RandomVal :type "Float (double-precision)"))
  (bind _values (`BlueprintMapLibrary.Map_Values` StringMap))
  (for _array_element _values
    (set `local.RunningSum` (+ _array_element (`local.RunningSum`))))
  (set `local.RandomVal` (`KismetMathLibrary.RandomFloatInRange` 0.0 (`local.RunningSum`)))
  (bind _keys (`BlueprintMapLibrary.Map_Keys` StringMap))
  (for _array_element_2 _keys
    (bind _value (`BlueprintMapLibrary.Map_Find` StringMap _array_element_2))
    (if (< (`local.RandomVal`) _value)
      (return _array_element_2)
      (else
        (set `local.RandomVal` (- (`local.RandomVal`) _value))))))

(fn `RandomChanceBool`
  (params (ChanceToReturnTrue :type "Float (double-precision)"))
  (returns (Return :type Boolean))
  (return (>= ChanceToReturnTrue (`KismetMathLibrary.RandomFloatInRange` 0.0 100.0))))