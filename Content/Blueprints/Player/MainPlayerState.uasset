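; MainPlayerState is a player state Blueprint that tracks the corpses a player leaves behind and caps how many exist in the world.
; AddCorpseToQueue appends each new corpse to PlayerCorpses; once the count exceeds CorpseLimit, it destroys the oldest valid corpse and removes that entry, forming a first-in, first-out queue.
; The reset event only calls its parent implementation, and the construction script is empty.
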(event `self.K2_OnReset`
  (`parent.K2_OnReset`))

(fn `AddCorpseToQueue`
  (params (NewCorpse :type "Actor Object Reference"))
  (bind _playercorpses (`self.PlayerCorpses`))
  (bind _playercorpses_2 (`self.PlayerCorpses`))
  (bind _output (`|GetArrayItem` _playercorpses))
  (`KismetArrayLibrary.Array_Add` _playercorpses_2 NewCorpse)
  (if (> (`KismetArrayLibrary.Array_Length` _playercorpses_2) (`self.CorpseLimit`))
    (`/Engine/EditorBlueprintResources/StandardMacros.IsValid` _output
      (:`Is Valid`
        (`self.K2_DestroyActor` _output))
      (:`Is Not Valid`
        _))
    (`KismetArrayLibrary.Array_Remove` _playercorpses)))

(fn `UserConstructionScript`)