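; Player controller for a multiplayer game, handling first spawn, possession, HUD, escape menu, underwater audio and disconnection to the main menu.
; It owns the hotbar inventory: add, remove and drop events update item slots, and ServerSetNewSelectedIndex toggles each item's Active state with forced net updates.
; On possess, a scene capture attaches to the pawn for the tab menu, whose toggle logic is unwired.
; Numpad keys trigger debug displays and simulated lag.
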(event `ServerNewPlayerPossessed`
  (params (Pawn :type "Pawn Object Reference"))
  (`|ExecutionSequence`
    (:`then_0`
      (bind _asmain_player_character (cast `/Game/Blueprints/Player/MainPlayerCharacter` Pawn))
      (bind _output_get (set `self.PlayerRef` _asmain_player_character))
      (`/Game/Blueprints/Player/MainPlayerCharacter.OwnerSetControlRotation` :`self` _output_get))
    (:`then_1`
      (`self.ServerSetNewSelectedIndex` (`self.SelectedIndex`)))))

(event `self.ReceiveBeginPlay`
  (set `self.GameStateRef` (cast `/Game/Blueprints/System/MainGameState` (`GameplayStatics.GetGameState`) :!pure true))
  (if (`self.IsLocalPlayerController`)
    (`|ExecutionSequence`
      (:`then_0`
        (bind _returnvalue (`|CreateWidget` "/Game/UI/W_PlayerHUD.W_PlayerHUD_C" self))
        (set `self.PlayerHUDRef` _returnvalue)
        (`UserWidget.AddToViewport` (`self.PlayerHUDRef`) 0))
      (:`then_1`
        (`self.ServerSpawnPlayerForFirstTime`)
        (bind _returnvalue_2 (`GameplayStatics.SpawnSound2D` "/Game/Audio/Ambient_Audio/UnderwaterAmbience.UnderwaterAmbience" 0.01 1.0 0.0 null))
        (set `self.UnderwaterAmbience` _returnvalue_2)))))

(event `self.ReceivePossess`
  (params (PossessedPawn :type "Pawn Object Reference"))
  ;[1 1 1] Tab Menu Capture Stuff
  (`|ExecutionSequence`
    (:`then_0`
      (`self.OwningClientOnPossess` PossessedPawn))
    (:`then_1`
      (`self.PlayerRef` ; This bit is necessary because idk how to assign the PlayerRef when the player first spawns, through the RestartPlayer node
        (:`then`)
        (:`else`
          (bind _asmain_player_character (cast `/Game/Blueprints/Player/MainPlayerCharacter` PossessedPawn))
          (set `self.PlayerRef` _asmain_player_character))))))

(event `ServerSpawnPlayerForFirstTime`
  (`GameModeBase.RestartPlayer` (`GameplayStatics.GetGameMode`) self))

(event `RemoveItem`
  (params (Item :type "/Game/Blueprints/Items/Item_Base Object Reference") (DestroyRemovedItem :type Boolean))
  (`|ExecutionSequence`
    (:`then_0`
      (for (_array_element _array_index) (`self.HotbarItems`)
        (if (== _array_element Item)
          (`KismetArrayLibrary.Array_Set` (`self.HotbarItems`) _array_index)
          (set `/Game/Blueprints/Items/Item_Base.Active` false Item) ; This is necessary for making the item inactive once a player sets it as their clicked item
          (break))))
    (:`then_1`
      (`self.ServerSetNewSelectedIndex` (`self.SelectedIndex`))
      (if DestroyRemovedItem
        (`self.K2_DestroyActor` Item)))))

(event `AddAndEquipItem`
  (params (NewItem :type "/Game/Blueprints/Items/Item_Base Object Reference"))
  (bind _emptyslotindex (`self.FindEmptyHotbarSlot`))
  (if (!= _emptyslotindex -1)
    (`KismetArrayLibrary.Array_Set` (`self.HotbarItems`) _emptyslotindex NewItem)
    (set `/Game/Blueprints/Items/Item_Base.MPC` self NewItem)
    (set `/Game/Blueprints/Items/Item_Base.PlayerRef` (`self.PlayerRef`) NewItem)
    (set `/Game/Blueprints/Items/Item_Base.Active` false NewItem) ; Necessary to set the visibility of the item, incase we have a 2h item or something
    (`self.ServerSetNewSelectedIndex` _emptyslotindex)))

(event `ServerItemSwap`
  (params (SwapNext :type Boolean))
  (if SwapNext
    (`self.ServerSetNewSelectedIndex` (`self.GetNextHotbarIndex`))
    (else
      (`self.ServerSetNewSelectedIndex` (`self.GetPrevHotbarIndex`)))))

(event `InputAction|NextItem`
  (params (Key :type "Key Structure"))
  (:`Pressed`
    (if (and (not (`KismetSystemLibrary.IsValid` null)) false)
      (`self.ServerItemSwap` true))))

(event `InputAction|PrevItem`
  (params (Key :type "Key Structure"))
  (:`Pressed`
    (if (and (not (`KismetSystemLibrary.IsValid` null)) false)
      (`self.ServerItemSwap` false))))

(event `ServerDropItem`
  (params (Item :type "/Game/Blueprints/Items/Item_Base Object Reference") (SpawnTransform :type "Transform Structure") (ThrowForce :type "Vector Structure"))
  (`/Game/Blueprints/Items/Item_Base.DropItem` Item SpawnTransform ThrowForce)
  (`self.RemoveItem` Item))

(event `AddItemAtIndex`
  (params (ItemBase :type "/Game/Blueprints/Items/Item_Base Object Reference") (Index :type Integer))
  (bind _selectedindex (`self.SelectedIndex`))
  (`KismetArrayLibrary.Array_Set` (`self.HotbarItems`) Index ItemBase)
  (set `self.HotbarItems` (`self.HotbarItems`))
  (set `/Game/Blueprints/Items/Item_Base.MPC` self ItemBase)
  (set `/Game/Blueprints/Items/Item_Base.PlayerRef` (`self.PlayerRef`) ItemBase)
  (set `/Game/Blueprints/Items/Item_Base.Active` false ItemBase)
  (if (== Index _selectedindex)
    (`self.ServerSetNewSelectedIndex` _selectedindex)))

(event `ServerSetNewSelectedIndex`
  (params (NewIndex :type Integer))
  (bind _output (`|GetArrayItem` (`self.HotbarItems`) NewIndex))
  (bind _output_2 (`|GetArrayItem` (`self.HotbarItems`) (`self.SelectedIndex`)))
  (`|ExecutionSequence`
    (:`then_0`
      (`/Engine/EditorBlueprintResources/StandardMacros.IsValid` _output_2
        (:`Is Valid`
          (`self.PlayerRef`
            (:`then`
              (set `/Game/Blueprints/Items/Item_Base.Active` false _output_2)
              (`self.ForceNetUpdate` _output_2))
            (:`else`)))))
    (:`then_1`
      (set `self.SelectedIndex` NewIndex))
    (:`then_2`
      (`/Engine/EditorBlueprintResources/StandardMacros.IsValid` _output
        (:`Is Valid`
          (`self.PlayerRef`
            (:`then`
              (set `/Game/Blueprints/Items/Item_Base.Active` true _output)
              (`self.ForceNetUpdate` _output))
            (:`else`)))
        (:`Is Not Valid`
          (bind _playerref (`self.PlayerRef`)
            (:`then`
              (`/Game/Blueprints/Player/MainPlayerCharacter.MultiResetFPPAnims` _playerref))
            (:`else`)))))))

(event `OwningClientOnPossess`
  (params (PossessedPawn :type "Pawn Object Reference"))
  (bind _tabmenucapture (`self.TabMenuCapture`))
  ;[1 1 1] Tab Menu Capture Stuff
  (bind _tabmenucapturetransform (message `/Game/Blueprints/Player/BPI_Character.GetTabMenuCaptureTransform` PossessedPawn))
  (`SceneComponent.K2_SetRelativeTransform` _tabmenucapture _tabmenucapturetransform false true)
  (`SceneComponent.K2_AttachToComponent` _tabmenucapture (`Actor.RootComponent` PossessedPawn) "None" "KeepRelative" "KeepRelative" "KeepRelative" true)
  (set `SceneCaptureComponent.ShowOnlyActors` (`|MakeArray` PossessedPawn :!type "Actor Object Reference") _tabmenucapture))

(event `InputAction|Pause`
  (params (Key :type "Key Structure"))
  ;[1 1 1] Escape menu
  (:`Pressed`
    (bind _returnvalue (`|CreateWidget` "/Game/UI/W_EscapeMenu.W_EscapeMenu_C" null self))
    (`UserWidget.AddToViewport` _returnvalue 0)))

(event `Key|Tab`
  (params (Key :type "Key Structure"))
  ;[1 1 1] Tab menu
)

(event `Key|NumPadOne`
  (params (Key :type "Key Structure"))
  ;[1 1 1] Debug stuff
  (:`Pressed`
    (`KismetSystemLibrary.ExecuteConsoleCommand` "stat fps" null)))

(event `Key|NumPadTwo`
  (params (Key :type "Key Structure"))
  ;[1 1 1] Debug stuff
  (:`Pressed`
    (`KismetSystemLibrary.ExecuteConsoleCommand` "show COLLISION" null)))

(event `Key|NumPadThree`
  (params (Key :type "Key Structure"))
  ;[1 1 1] Debug stuff
  (:`Pressed`
    (`self.MultiEnableLag`)))

(event `Key|NumPadFour`
  (params (Key :type "Key Structure"))
  ;[1 1 1] Debug stuff
  (:`Pressed`
    (`self.MultiDisableLag`)))

(event `MultiEnableLag`
  ;[1 1 1] Debug stuff
  (`KismetSystemLibrary.ExecuteConsoleCommand` "Net PktLoss=1" null)
  (`KismetSystemLibrary.ExecuteConsoleCommand` "Net PktOrder=0" null)
  (`KismetSystemLibrary.ExecuteConsoleCommand` "Net PktDup=0" null)
  (`KismetSystemLibrary.ExecuteConsoleCommand` "Net PktLag=500" null)
  (`KismetSystemLibrary.ExecuteConsoleCommand` "Net PktLagVariance=0" null)
  (`KismetSystemLibrary.ExecuteConsoleCommand` "p.netshowcorrections 1" null))

(event `MultiDisableLag`
  ;[1 1 1] Debug stuff
  (`KismetSystemLibrary.ExecuteConsoleCommand` "Net PktLoss=0" null)
  (`KismetSystemLibrary.ExecuteConsoleCommand` "Net PktOrder=0" null)
  (`KismetSystemLibrary.ExecuteConsoleCommand` "Net PktDup=0" null)
  (`KismetSystemLibrary.ExecuteConsoleCommand` "Net PktLag=0" null)
  (`KismetSystemLibrary.ExecuteConsoleCommand` "Net PktLagVariance=0" null)
  (`KismetSystemLibrary.ExecuteConsoleCommand` "p.netshowcorrections 0" null))

(event `Disconnect`
  ;[1 1 1] When a player gets kicked
  (`|ExecutionSequence`
    (:`then_0`
      (`/Engine/EditorBlueprintResources/StandardMacros.IsValid` (`self.K2_GetPawn`)))
    (:`then_1`
      (`GameplayStatics.OpenLevel` "MainMenu")
      (`DestroySessionCallbackProxy.DestroySession` self))))

(event `SetUnderwaterSoundMix`
  (params (Underwater :type Boolean))
  (if Underwater
    (`GameplayStatics.PushSoundMixModifier` "/Game/Audio/UnderwaterSoundMix.UnderwaterSoundMix")
    (`AudioComponent.SetVolumeMultiplier` (`self.UnderwaterAmbience`) 1.0)
    (else
      (`GameplayStatics.ClearSoundMixModifiers`)
      (`AudioComponent.SetVolumeMultiplier` (`self.UnderwaterAmbience`) 0.01))))

(fn `FindEmptyHotbarSlot`
  (returns (EmptySlotIndex :type Integer))
  (locals (foundEmptySlot :type Boolean))
  (for (_array_element _array_index) (`self.HotbarItems`)
    (`/Engine/EditorBlueprintResources/StandardMacros.IsValid` _array_element
      (:`Is Not Valid`
        (set `local.foundEmptySlot` true)
        (break))))
  (if (`local.foundEmptySlot`)
    (return _array_index)
    (else
      (return -1))))

(fn `GetNextHotbarIndex`
  (returns (Return :type Integer))
  (bind _selectedindex (`self.SelectedIndex`))
  (bind _returnvalue (`KismetArrayLibrary.Array_LastIndex` (`self.HotbarItems`)))
  (if (== _selectedindex _returnvalue)
    ;[1 1 1] Otherwise, cycle back to zero
    (return 0)
    (else
      ;[1 1 1] If not, just go to the next item
      (return (`KismetMathLibrary.Clamp` (+ _selectedindex 1) 0 _returnvalue)))))

(fn `GetPlayerName`
  (returns (PlayerName :type String))
  (return (`PlayerState.GetPlayerName` (`self.PlayerState`))))

(fn `GetPrevHotbarIndex`
  (returns (Return :type Integer))
  (bind _selectedindex (`self.SelectedIndex`))
  (bind _returnvalue (`KismetArrayLibrary.Array_LastIndex` (`self.HotbarItems`)))
  (if (== _selectedindex 0)
    ;[1 1 1] Otherwise, cycle to end of hotbar
    (return _returnvalue)
    (else
      ;[1 1 1] If not, just go to the previous weapon
      (return (`KismetMathLibrary.Clamp` (- _selectedindex 1) 0 _returnvalue)))))

(fn `GetSelectedItem`
  (returns (SelectedItem :type "/Game/Blueprints/Items/Item_Base Object Reference"))
  (`/Engine/EditorBlueprintResources/StandardMacros.IsValid` null
    (:`Is Valid`
      (return null))
    (:`Is Not Valid`
      (return (`|GetArrayItem` (`self.HotbarItems`) (`self.SelectedIndex`))))))

(fn `UserConstructionScript`)